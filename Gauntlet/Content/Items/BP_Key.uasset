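; BP_Key is a collectible key pickup that increments a shared key count and destroys itself.
; Its WorldCollision component finds the KeyManager by overlap, caches the reference, then destroys itself.
; A Box overlap ignores Enemy-tagged actors, prints the other actor's name and grants the key only when that display name is "DefaultPawn", a temporary player check.
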(event `self.Box.OnComponentBeginOverlap`
  (params (OverlappedComponent :type "PrimitiveComponent Object Reference") (OtherActor :type "Actor Object Reference") (OtherComp :type "PrimitiveComponent Object Reference") (OtherBodyIndex :type Integer) (bFromSweep :type Boolean) (SweepResult :type "HitResult Structure (by ref)"))
  (bind _returnvalue (`KismetSystemLibrary.GetDisplayName` OtherActor))
  (bind _keymanager (`self.keyManager`))
  ;[1 1 1] Ignore Enemy Collision
  (if (not (`self.ActorHasTag` OtherActor "Enemy"))
    ;[1 1 1] Checks if I'ts  Player (For now Defautl Pawn)
    (`KismetSystemLibrary.PrintString` _returnvalue)
    (if (== _returnvalue "DefaultPawn")
      ;[1 1 1] Adds to Key Manager
      (set `/Game/Items/KeyManager.KeyAmount` (+ (`/Game/Items/KeyManager.KeyAmount` _keymanager) 1) _keymanager)
      (`self.K2_DestroyActor`))))

(event `self.World Collision.OnComponentBeginOverlap`
  (params (OverlappedComponent :type "PrimitiveComponent Object Reference") (OtherActor :type "Actor Object Reference") (OtherComp :type "PrimitiveComponent Object Reference") (OtherBodyIndex :type Integer) (bFromSweep :type Boolean) (SweepResult :type "HitResult Structure (by ref)"))
  ;[1 1 1] Gets Key  Manager
  (bind _askey_manager (cast `/Game/Items/KeyManager` OtherActor))
  (set `self.keyManager` _askey_manager)
  (`ActorComponent.K2_DestroyComponent` (`self.World Collision`)))

(fn `UserConstructionScript`)