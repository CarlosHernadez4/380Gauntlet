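; Enemy that chases pawns it sees and fires projectiles at them, losing one health per hit until destroyed.
; PawnSensing stores the target; Tick runs AI MoveTo to the Stats range, where attacks spawn BP_Projectile on a timer-reset cooldown.
; A sphere overlap records heroes by tag for per-tick distance tracking, though only Elf's distance is wired.
; Random-interval invisibility toggles visibility and collision, but its call here is disconnected.
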(event `Turn on Invisibility`
  (bind _returnvalue (`KismetMathLibrary.RandomFloatInRange` 0.5 3.0))
  (bind _capsulecomponent (`self.CapsuleComponent`))
  ;[1 1 1] Invisibility
  (`SceneComponent.SetVisibility` _capsulecomponent false true)
  (`PrimitiveComponent.SetCollisionEnabled` _capsulecomponent "NoCollision")
  (`KismetSystemLibrary.Delay` _returnvalue)
  (`SceneComponent.SetVisibility` _capsulecomponent true true)
  (`PrimitiveComponent.SetCollisionEnabled` _capsulecomponent "QueryAndPhysics")
  (`KismetSystemLibrary.K2_SetTimer` null "Turn on Invisibility" _returnvalue true))

(event `self.PawnSensing.OnHearNoise`
  (params (Instigator :type "Pawn Object Reference") (Location :type "Vector Structure (by ref)") (Volume :type "Float (single-precision)")))

(event `self.ReceiveTick`
  (params (DeltaSeconds :type "Float (single-precision)"))
  ;[1 1 1] Update - Move
  (if (`self.isSeeingPlayer`)
    (`self.Follow Player`)
    (else
      (`MovementComponent.StopMovementImmediately` (`self.CharacterMovement`))))
  (`self.Get Distance`))

(event `self.PawnSensing.OnSeePawn`
  (params (Pawn :type "Pawn Object Reference"))
  ;[1 1 1] On See Pawn
  (set `self.Pawn` Pawn)
  (set `self.isSeeingPlayer` true))

(event `self.CapsuleComponent.OnComponentBeginOverlap`
  (params (OverlappedComponent :type "PrimitiveComponent Object Reference") (OtherActor :type "Actor Object Reference") (OtherComp :type "PrimitiveComponent Object Reference") (OtherBodyIndex :type Integer) (bFromSweep :type Boolean) (SweepResult :type "HitResult Structure (by ref)")))

(event `self.ReceiveBeginPlay`)

(event `Follow Player`
  ;[1 1 1] Follow Player
  (if (`self.isSeeingPlayer`)
    (`|AIMoveTo` self (`self.K2_GetActorLocation` (`self.Pawn`)) null (`.Range_15_AE6CF24E42D6FB128A62ADA5D6FE1211` (break `/Game/Enemies/Enum/S_EnemyStats` (`self.Stats`)))
      (:`then`
        (`self.Attack` :!label _label))
      (:`OnSuccess`
        (`KismetSystemLibrary.PrintString` "Success")
        (set `self.InRange` true)
        (goto _label))
      (:`OnFail`
        (`KismetSystemLibrary.PrintString` "Fail")
        (set `self.InRange` false)))
    (else
      (set `self.isSeeingPlayer` false))))

(event `Damage Enemy`
  (bind _stats (`self.Stats`))
  (bind ((`Health_12_D48A8CF14ACF631928A12998109E21C0` _health)) (break `/Game/Enemies/Enum/S_EnemyStats` _stats))
  ;[1 1 1] Damage Enemy
  (setmembers `/Game/Enemies/Enum/S_EnemyStats` :`StructRef` _stats :`Health` (- _health 1))
  (if (<= _health 0)
    (`self.K2_DestroyActor`)))

(event `Attack`
  ;[1 1 1] Attack
  (if (`self.InRange`)
    (if (== (`self.AttackOnCD`) false)
      (set `self.AttackOnCD` true)
      (`|SpawnActorFromClass` "/Game/Enemies/Blueprints/BP_Projectile.BP_Projectile_C" (`SceneComponent.K2_GetComponentToWorld` (`self.Projectile Spawn Pos`)) "AdjustIfPossibleButAlwaysSpawn" "OverrideRootScale" null null)
      (`KismetSystemLibrary.K2_SetTimer` null "ResetCD" (`self.AttackSpeed`)))))

(event `ResetCD`
  ;[1 1 1] Attack
  (set `self.AttackOnCD` false))

(event `Delete Sphere Collider`
  ;[1 1 1] Delete Sphere Comp
  (`KismetSystemLibrary.Delay` 0.5)
  (`ActorComponent.K2_DestroyComponent` (`self.Sphere`)))

(event `self.Sphere.OnComponentBeginOverlap`
  (params (OverlappedComponent :type "PrimitiveComponent Object Reference") (OtherActor :type "Actor Object Reference") (OtherComp :type "PrimitiveComponent Object Reference") (OtherBodyIndex :type Integer) (bFromSweep :type Boolean) (SweepResult :type "HitResult Structure (by ref)"))
  ;[1 1 1] Set Player Vars
  (if (`self.ActorHasTag` OtherActor "Elf")
    (set `self.Elf` OtherActor)
    (elif (`self.ActorHasTag` OtherActor "Valk")
      (set `self.Valk` OtherActor)
      (elif (`self.ActorHasTag` "Wizard")
        (set `self.Wizard` OtherActor)
        (elif (`self.ActorHasTag` "Warrior")
          (set `self.Warrior` OtherActor))))))

(event `Get Distance`
  ;[1 1 1] SEt Distnances\
  (bind _aself_bp (cast `/Game/Players/Elf_Bp` (`self.Elf`)))
  (setmembers `/Game/Enemies/Enum/S_Distance` :`StructRef` (`self.Distances`) :`DisValk` (`self.GetDistanceTo` self null) :`DisWarrior` (`self.GetDistanceTo` self null) :`DisWizard` (`self.GetDistanceTo` self null) :`DisElf` (`self.GetDistanceTo` self _aself_bp)))

(fn `UserConstructionScript`)