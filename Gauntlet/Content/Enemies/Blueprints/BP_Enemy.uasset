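; BP_Enemy is an enemy that chases a pawn it spots through PawnSensing.
; Seeing any pawn sets IsSeeingPlayer, which is never cleared here, and calls FollowPlayer.
; FollowPlayer uses AIMoveTo toward that pawn with Range as the acceptance radius, printing success or failure as debug text.
; BeginPlay, Tick and overlap events are empty, and leftover SimpleMoveToLocation and MoveComponentTo nodes never run.
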(event `self.PawnSensing.OnSeePawn`
  (params (Pawn :type "Pawn Object Reference"))
  (set `self.isSeeingPlayer` true)
  (`self.Follow Player`))

(event `Follow Player`
  (if (`self.isSeeingPlayer`)
    (`|AIMoveTo` self (0.0 0.0 0.0) (stale `self.PawnSensing.OnSeePawn` Pawn) (`self.Range`)
      (:`OnSuccess`
        (`KismetSystemLibrary.PrintString` "Success"))
      (:`OnFail`
        (`KismetSystemLibrary.PrintString` "Fail")))))

(fn `UserConstructionScript`)