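; TestPlayer2 is a test player Blueprint under Enemies that reads WASD input into a direction vector.
; BeginPlay enables input, then each key press adds a unit offset on X or Y to KeyPressed and each release subtracts it, so held keys combine.
; A swept capsule move by that vector from the actor location is present but unwired, so the graph never moves the actor.
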(event `self.ReceiveBeginPlay`
  (`self.EnableInput` null))

(event `Key|W`
  (params (Key :type "Key Structure"))
  (:`Pressed`
    (set `self.key pressed` (+ (0.0 1.0 0.0) (`self.key pressed`))))
  (:`Released`
    (set `self.key pressed` (+ (0.0 -1.0 0.0) (`self.key pressed`)))))

(event `Key|S`
  (params (Key :type "Key Structure"))
  (:`Pressed`
    (set `self.key pressed` (+ (0.0 -1.0 0.0) (`self.key pressed`))))
  (:`Released`
    (set `self.key pressed` (+ (0.0 1.0 0.0) (`self.key pressed`)))))

(event `Key|A`
  (params (Key :type "Key Structure"))
  (:`Pressed`
    (set `self.key pressed` (+ (1.0 0.0 0.0) (`self.key pressed`))))
  (:`Released`
    (set `self.key pressed` (+ (-1.0 0.0 0.0) (`self.key pressed`)))))

(event `Key|D`
  (params (Key :type "Key Structure"))
  (:`Pressed`
    (set `self.key pressed` (+ (-1.0 0.0 0.0) (`self.key pressed`))))
  (:`Released`
    (set `self.key pressed` (+ (1.0 0.0 0.0) (`self.key pressed`)))))

(fn `UserConstructionScript`)