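; BP_Block is an enemy spawner block that spawns a BP_EnemyFollow on BeginPlay and then repeatedly at the SpawnRate interval.
; Each spawn takes random X and Y within a box sized by the SpehreSpawnRange sphere's radius, and Z from the Cube.
; SpawnEnemy re-arms its own looping timer by function name on every call.
; An unconnected SpawnType branch chain for enemy kinds like Ghost and Grunt never runs.
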(event `self.ReceiveBeginPlay`
  (`self.Spawn Enemy`))

(event `Spawn Enemy`
  (bind _spehre_spawn_range (`self.Spehre Spawn Range`))
  (bind (_returnvalue_x _returnvalue_y _returnvalue_z) (`KismetMathLibrary.BreakVector` (`SceneComponent.K2_GetComponentLocation` (`self.Cube`))))
  (bind (_returnvalue_x_2 _returnvalue_y_2) (`KismetMathLibrary.BreakVector` (`KismetMathLibrary.RandomPointInBoundingBox` (`SceneComponent.K2_GetComponentLocation` _spehre_spawn_range) (`KismetMathLibrary.Conv_DoubleToVector` (`SphereComponent.GetScaledSphereRadius` _spehre_spawn_range)))))
  (`|SpawnActorFromClass` "/Game/Enemies/Blueprints/BP_EnemyFollow.BP_EnemyFollow_C" (`KismetMathLibrary.MakeTransform` (`KismetMathLibrary.MakeVector` _returnvalue_x_2 _returnvalue_y_2 _returnvalue_z)) "AdjustIfPossibleButDontSpawnIfColliding" "OverrideRootScale" null null)
  (`KismetSystemLibrary.K2_SetTimer` null "Spawn Enemy" (`self.SpawnRate`) true))

(fn `UserConstructionScript`)