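; BP_Bones is a destructible bone-pile spawner that periodically creates BP_Ghost enemies.
; SpawnEnemy runs on BeginPlay and on a SpawnRate timer, placing ghosts at random X/Y within the spawn sphere's bounding box at the cube's height and passing on its level.
; Overlaps from three projectile classes destroy the projectile and remove one health, destroying the spawner at zero.
; An unconnected SpawnType branch chain for other enemy types never runs.
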(event `self.ReceiveBeginPlay`
  (`self.Spawn Enemy`))

(event `Spawn Enemy`
  (bind _spehre_spawn_range (`self.Spehre Spawn Range`))
  (bind (_returnvalue_x _returnvalue_y _returnvalue_z) (`KismetMathLibrary.BreakVector` (`SceneComponent.K2_GetComponentLocation` (`self.Cube`))))
  (bind (_returnvalue_x_2 _returnvalue_y_2) (`KismetMathLibrary.BreakVector` (`KismetMathLibrary.RandomPointInBoundingBox` (`SceneComponent.K2_GetComponentLocation` _spehre_spawn_range) (`KismetMathLibrary.Conv_DoubleToVector` (`SphereComponent.GetScaledSphereRadius` _spehre_spawn_range)))))
  (bind _returnvalue (`|SpawnActorFromClass` "/Game/Carlos/Enemies/Blueprints/BP_Ghost.BP_Ghost_C" (`KismetMathLibrary.MakeTransform` (`KismetMathLibrary.MakeVector` _returnvalue_x_2 _returnvalue_y_2 _returnvalue_z)) "AdjustIfPossibleButAlwaysSpawn" "OverrideRootScale" null (struct) null))
  (bind ((`EnemyType_2_ED4A4E914A448F8791ED5798B541B178` _enemytype) (`Health_12_D48A8CF14ACF631928A12998109E21C0` _health) (`Damage_14_E6BD71484CDE36F86E904CAA5C2D6F21` _damage) (`Range_15_AE6CF24E42D6FB128A62ADA5D6FE1211` _range)) (break `/Game/Carlos/Enemies/Enum/S_EnemyStats` (`/Game/Carlos/Enemies/Blueprints/BP_Ghost.Stats` _returnvalue)))
  (set `/Game/Carlos/Enemies/Blueprints/BP_Ghost.Stats` (make `/Game/Carlos/Enemies/Enum/S_EnemyStats` _enemytype _health (`.Level_13_B0432F0149067147026B04B503074291` (break `/Game/Carlos/Enemies/Enum/S_EnemyStats` (`self.BlockStat`))) _damage _range) _returnvalue)
  (`KismetSystemLibrary.K2_SetTimer` null "Spawn Enemy" (`self.SpawnRate`) true))

(event `self.Box.OnComponentBeginOverlap`
  (params (OverlappedComponent :type "PrimitiveComponent Object Reference") (OtherActor :type "Actor Object Reference") (OtherComp :type "PrimitiveComponent Object Reference") (OtherBodyIndex :type Integer) (bFromSweep :type Boolean) (SweepResult :type "HitResult Structure (by ref)"))
  ;[1 1 1] Detect Projectile
  (bind _asbp_projectile (cast `/Game/Carlos/Enemies/Blueprints/BP_Projectile` OtherActor)
    (:`then`
      (`self.Damage Bones`)
      (`self.K2_DestroyActor` _asbp_projectile))
    (:`CastFailed`
      (bind _asbp_projectal (cast `/Game/Players/Bp_Projectal` OtherActor)
        (:`then`
          (`self.Damage Bones`)
          (`self.K2_DestroyActor` _asbp_projectal))
        (:`CastFailed`
          (bind _asbp_lobber_projectile (cast `/Game/Carlos/Enemies/Blueprints/BP_LobberProjectile` OtherActor))
          (`self.Damage Bones`)
          (`self.K2_DestroyActor` _asbp_lobber_projectile))))))

(event `Damage Bones`
  (bind _blockstat (`self.BlockStat`))
  (bind ((`Health_12_D48A8CF14ACF631928A12998109E21C0` _health)) (break `/Game/Carlos/Enemies/Enum/S_EnemyStats` _blockstat))
  ;[1 1 1] Damage Bones
  (setmembers `/Game/Carlos/Enemies/Enum/S_EnemyStats` :`StructRef` _blockstat :`Health` (- _health 1))
  (if (<= _health 0)
    (`self.K2_DestroyActor`)))

(fn `UserConstructionScript`)