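; Base enemy prototype that reacts to nearby actors and sighted pawns with simple rotation and movement.
; A Sphere overlap toggles InRadius, and Tick then applies the Rotator variable to the Box, though the look-at calculation for Rotator is disconnected.
; PawnSensing prints a debug string and calls MoveForward, which nudges the parent actor's root along relative X without sweeping.
; Character filtering, input toggling and timeline-driven movement are unwired.
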(event OnSeePawn(PawnSensing)
  (params (Pawn :type Pawn%20Object%20Reference))
  (Development|PrintString "forward")
  (CallFunction|MoveForward))

(event OnComponentBeginOverlap(Sphere)
  (params (OverlappedComponent :type Primitive%20Component%20Object%20Reference) (OtherActor :type Actor%20Object%20Reference) (OtherComp :type Primitive%20Component%20Object%20Reference) (OtherBodyIndex :type Integer) (bFromSweep :type Boolean) (SweepResult :type Hit%20Result%20Structure%20%28by%20ref%29))
  (Variables|Default|SetIn%20Radius true))

(event OnComponentEndOverlap(Sphere)
  (params (OverlappedComponent :type Primitive%20Component%20Object%20Reference) (OtherActor :type Actor%20Object%20Reference) (OtherComp :type Primitive%20Component%20Object%20Reference) (OtherBodyIndex :type Integer))
  (Variables|Default|SetIn%20Radius false))

(event Custom|MoveForward
  (Transformation|AddRelativeLocation (Variables|/Script/Engine.Actor|GetRootComponent (Actor|GetParentActor)) "1.000000, 0, 0" false false))

(event EventBeginPlay)

(event Collision|EventActorBeginOverlap
  (params (OtherActor :type Actor%20Object%20Reference)))

(event EventTick
  (params (DeltaSeconds :type Float%20%28single-precision%29))
  (if (Variables|Default|GetIn%20Radius)
    (Transformation|SetRelativeRotation (Variables|Default|GetBox) (stale _output_get) false false)))

(fn ConstructionScript)