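; BP_Ghost is a suicide-attack enemy that chases a seen pawn and damages the player.
; PawnSensing stores the pawn and latches a seeing flag, so Tick reissues AI MoveTo toward it using the stats range.
; When in range or on Box overlap with the player, it deals level-scaled damage and destroys itself.
; Projectile overlaps on the Box reduce its stats-struct health, destroying it at zero.
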(event `self.ReceiveTick`
  (params (DeltaSeconds :type "Float (single-precision)"))
  ;[1 1 1] Update - Move
  (if (`self.isSeeingPlayer`)
    (`self.Follow Player`)
    (else
      (`MovementComponent.StopMovementImmediately` (`self.CharacterMovement`)))))

(event `self.PawnSensing.OnSeePawn`
  (params (Pawn :type "Pawn Object Reference"))
  ;[1 1 1] On See Pawn
  (set `self.Pawn` Pawn)
  (set `self.isSeeingPlayer` true))

(event `self.ReceiveBeginPlay`)

(event `Follow Player`
  ;[1 1 1] Follow Player
  (if (`self.isSeeingPlayer`)
    (`|AIMoveTo` self (`self.K2_GetActorLocation` (`self.Pawn`)) null (`.Range_15_AE6CF24E42D6FB128A62ADA5D6FE1211` (break `/Game/Carlos/Enemies/Enum/S_EnemyStats` (`self.Stats`)))
      (:`then`
        (`self.Attack` :!label _label))
      (:`OnSuccess`
        (`KismetSystemLibrary.PrintString` "Success")
        (set `self.InRange` true)
        (goto _label))
      (:`OnFail`
        (set `self.InRange` false)))
    (else
      (set `self.isSeeingPlayer` false))))

(event `Damage Enemy`
  (bind _stats (`self.Stats`))
  (bind ((`Health_12_D48A8CF14ACF631928A12998109E21C0` _health)) (break `/Game/Carlos/Enemies/Enum/S_EnemyStats` _stats))
  ;[1 1 1] Damage Enemy
  (setmembers `/Game/Carlos/Enemies/Enum/S_EnemyStats` :`StructRef` _stats :`Health` (- _health 1))
  (if (<= _health 0)
    (`self.K2_DestroyActor`)))

(event `self.CapsuleComponent.OnComponentBeginOverlap`
  (params (OverlappedComponent :type "PrimitiveComponent Object Reference") (OtherActor :type "Actor Object Reference") (OtherComp :type "PrimitiveComponent Object Reference") (OtherBodyIndex :type Integer) (bFromSweep :type Boolean) (SweepResult :type "HitResult Structure (by ref)")))

(event `Attack`
  ;[1 1 1] Attack
  (if (`self.InRange`)
    (`self.Damage Player`)
    (`self.K2_DestroyActor`)))

(event `Damage Player`
  (bind ((`Level_13_B0432F0149067147026B04B503074291` _level) (`Damage_14_E6BD71484CDE36F86E904CAA5C2D6F21` _damage)) (break `/Game/Carlos/Enemies/Enum/S_EnemyStats` (`self.Stats`)))
  (bind _asbp_player_class (cast `/Game/Players/Bp_Player_Class` (`self.Pawn`)))
  (set `/Game/Players/Bp_Player_Class.Hp` (- (`/Game/Players/Bp_Player_Class.Hp` _asbp_player_class) (* _level _damage)) _asbp_player_class))

(event `self.Box.OnComponentBeginOverlap`
  (params (OverlappedComponent :type "PrimitiveComponent Object Reference") (OtherActor :type "Actor Object Reference") (OtherComp :type "PrimitiveComponent Object Reference") (OtherBodyIndex :type Integer) (bFromSweep :type Boolean) (SweepResult :type "HitResult Structure (by ref)"))
  ;[1 1 1] Self Destruct
  (cast `/Game/Players/Bp_Player_Class` OtherActor
    (:`then`
      (`self.Damage Player`)
      (`self.K2_DestroyActor`))
    (:`CastFailed`
      (cast `/Game/Players/Bp_Projectal` OtherActor)
      (`self.Damage Enemy`))))

(fn `UserConstructionScript`)