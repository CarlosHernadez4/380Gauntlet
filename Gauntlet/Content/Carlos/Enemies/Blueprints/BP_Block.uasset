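; BP_Block is a destructible enemy spawner that spawns BP_Ghost actors at a looping SpawnRate.
; SpawnEnemy picks a random XY in a box sized by SpehreSpawnRange, uses the Cube's height, passes on the block's Level and arms its timer after a successful spawn.
; Projectile overlaps on Box destroy the projectile and call DamageBones, removing one Health and destroying the block at zero.
; A SpawnType branch chain is unconnected, so only ghosts spawn.
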(event `self.ReceiveBeginPlay`
  (`self.Spawn Enemy`))

(event `Spawn Enemy`
  (bind _spehre_spawn_range (`self.Spehre Spawn Range`))
  (bind (_returnvalue_x _returnvalue_y _returnvalue_z) (`KismetMathLibrary.BreakVector` (`SceneComponent.K2_GetComponentLocation` (`self.Cube`))))
  (bind (_returnvalue_x_2 _returnvalue_y_2) (`KismetMathLibrary.BreakVector` (`KismetMathLibrary.RandomPointInBoundingBox` (`SceneComponent.K2_GetComponentLocation` _spehre_spawn_range) (`KismetMathLibrary.Conv_DoubleToVector` (`SphereComponent.GetScaledSphereRadius` _spehre_spawn_range)))))
  (bind _returnvalue (`|SpawnActorFromClass` "/Game/Carlos/Enemies/Blueprints/BP_Ghost.BP_Ghost_C" (`KismetMathLibrary.MakeTransform` (`KismetMathLibrary.MakeVector` _returnvalue_x_2 _returnvalue_y_2 _returnvalue_z)) "AdjustIfPossibleButDontSpawnIfColliding" "OverrideRootScale" null (struct) null))
  (bind _asbp_ghost (cast `/Game/Carlos/Enemies/Blueprints/BP_Ghost` _returnvalue))
  (bind _structout (setmembers `/Game/Carlos/Enemies/Enum/S_EnemyStats` :`StructRef` (`/Game/Carlos/Enemies/Blueprints/BP_Ghost.Stats` _asbp_ghost) :`Level` (`.Level_13_B0432F0149067147026B04B503074291` (break `/Game/Carlos/Enemies/Enum/S_EnemyStats` (`self.BlockStat`)))))
  (`KismetSystemLibrary.K2_SetTimer` null "Spawn Enemy" (`self.SpawnRate`) true))

(event `self.Box.OnComponentBeginOverlap`
  (params (OverlappedComponent :type "PrimitiveComponent Object Reference") (OtherActor :type "Actor Object Reference") (OtherComp :type "PrimitiveComponent Object Reference") (OtherBodyIndex :type Integer) (bFromSweep :type Boolean) (SweepResult :type "HitResult Structure (by ref)"))
  ;[1 1 1] Detect Projectile
  (bind _asbp_projectile (cast `/Game/Carlos/Enemies/Blueprints/BP_Projectile` OtherActor)
    (:`then`
      (`self.Damage Bones`)
      (`self.K2_DestroyActor` _asbp_projectile))
    (:`CastFailed`
      (bind _asbp_projectal (cast `/Game/Players/Bp_Projectal` OtherActor))
      (`self.Damage Bones`)
      (`self.K2_DestroyActor` _asbp_projectal))))

(event `Damage Bones`
  (bind _blockstat (`self.BlockStat`))
  (bind ((`Health_12_D48A8CF14ACF631928A12998109E21C0` _health)) (break `/Game/Carlos/Enemies/Enum/S_EnemyStats` _blockstat))
  ;[1 1 1] Damage Bones
  (setmembers `/Game/Carlos/Enemies/Enum/S_EnemyStats` :`StructRef` _blockstat :`Health` (- _health 1))
  (if (<= _health 0)
    (`self.K2_DestroyActor`)))

(fn `UserConstructionScript`)