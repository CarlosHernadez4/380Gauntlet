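; BP_Death is a Death enemy that chases pawns spotted by PawnSensing and attacks in melee, with damage set by level.
; AIMoveTo feeds a timer-gated attack that subtracts player Hp and destroys the enemy if that Hp is 200 or below.
; Projectile overlaps remove one health, destroying it at zero.
; Until first sighting, Tick halts movement and runs unfinished player-distance tracking, whose player-reference setup is disconnected.
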(event `self.ReceiveTick`
  (params (DeltaSeconds :type "Float (single-precision)"))
  ;[1 1 1] Update - Move
  (if (not (`self.isSeeingPlayer`))
    (`MovementComponent.StopMovementImmediately` (`self.CharacterMovement`))
    (`self.Get Distance`)))

(event `self.PawnSensing.OnSeePawn`
  (params (Pawn :type "Pawn Object Reference"))
  ;[1 1 1] On See Pawn
  (set `self.Pawn` Pawn)
  (set `self.isSeeingPlayer` true)
  (`self.Follow Player`))

(event `self.ReceiveBeginPlay`
  (bind _stats (`self.Stats`))
  (bind ((`Level_13_B0432F0149067147026B04B503074291` _level)) (break `/Game/Carlos/Enemies/Enum/S_EnemyStats` _stats))
  ;[1 1 1] Set Level Damage
  (if (== _level 1)
    _
    (elif (== _level 2)
      (setmembers `/Game/Carlos/Enemies/Enum/S_EnemyStats` :`StructRef` _stats :`Damage` 8)
      (elif (== _level 3)
        (setmembers `/Game/Carlos/Enemies/Enum/S_EnemyStats` :`StructRef` _stats :`Damage` 10)))))

(event `Follow Player`
  ;[1 1 1] Follow Player
  (if (`self.isSeeingPlayer`)
    (`|AIMoveTo` self (`self.K2_GetActorLocation` (`self.Pawn`)) null (`.Range_15_AE6CF24E42D6FB128A62ADA5D6FE1211` (break `/Game/Carlos/Enemies/Enum/S_EnemyStats` (`self.Stats`)))
      (:`then`
        _)
      (:`OnSuccess`
        (`KismetSystemLibrary.PrintString` "Success")
        (set `self.InRange` true)))
    (`self.Attack`)
    (else
      (set `self.isSeeingPlayer` false))))

(event `Damage Enemy`
  (bind _stats (`self.Stats`))
  (bind ((`Health_12_D48A8CF14ACF631928A12998109E21C0` _health)) (break `/Game/Carlos/Enemies/Enum/S_EnemyStats` _stats))
  ;[1 1 1] Damage Enemy
  (setmembers `/Game/Carlos/Enemies/Enum/S_EnemyStats` :`StructRef` _stats :`Health` (- _health 1))
  (if (<= _health 0)
    (`self.K2_DestroyActor`)))

(event `Attack`
  ;[1 1 1] Attack
  (if (`self.InRange`)
    (if (== (`self.AttackOnCD`) false)
      (`KismetSystemLibrary.PrintString` "attack")
      (set `self.AttackOnCD` true)
      (`self.Damage Player`)
      (`KismetSystemLibrary.K2_SetTimer` null "ResetCD" (`self.AttackSpeed`)))))

(event `ResetCD`
  ;[1 1 1] Attack
  (set `self.AttackOnCD` false))

(event `Damage Player`
  (bind _asbp_player_class (cast `/Game/Players/Bp_Player_Class` (`self.Pawn`)))
  (bind _output_get (set `/Game/Players/Bp_Player_Class.Hp` (- (`/Game/Players/Bp_Player_Class.Hp` _asbp_player_class) (`.Damage_14_E6BD71484CDE36F86E904CAA5C2D6F21` (break `/Game/Carlos/Enemies/Enum/S_EnemyStats` (`self.Stats`)))) _asbp_player_class))
  (if (<= _output_get 200)
    (`self.K2_DestroyActor`)))

(event `Delete Sphere Collider`
  ;[1 1 1] Delete Sphere Comp
  (`KismetSystemLibrary.Delay` 0.5))

(event `self.CapsuleComponent.OnComponentBeginOverlap`
  (params (OverlappedComponent :type "PrimitiveComponent Object Reference") (OtherActor :type "Actor Object Reference") (OtherComp :type "PrimitiveComponent Object Reference") (OtherBodyIndex :type Integer) (bFromSweep :type Boolean) (SweepResult :type "HitResult Structure (by ref)"))
  (bind _stats (`self.Stats`))
  (bind ((`Health_12_D48A8CF14ACF631928A12998109E21C0` _health)) (break `/Game/Carlos/Enemies/Enum/S_EnemyStats` _stats))
  ;[1 1 1] Damage Enemy
  (`KismetSystemLibrary.PrintString` "Hello")
  (cast `/Game/Players/Bp_Projectal` OtherActor)
  (setmembers `/Game/Carlos/Enemies/Enum/S_EnemyStats` :`StructRef` _stats :`Health` (- _health 1))
  (if (<= _health 0)
    (`self.K2_DestroyActor`)))

(event `Get Distance`
  ;[1 1 1] SEt Distnances\
  (bind _asbp_player_class (cast `/Game/Players/Bp_Player_Class` (`self.Elf`)))
  (setmembers `/Game/Carlos/Enemies/Enum/S_Distance` :`StructRef` (`self.Distances`) :`DisValk` (`self.GetDistanceTo` self null) :`DisWarrior` (`self.GetDistanceTo` self null) :`DisWizard` (`self.GetDistanceTo` self null) :`DisElf` (`self.GetDistanceTo` self _asbp_player_class)))

(fn `UserConstructionScript`)