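; Ranged Lobber enemy that pursues a sensed pawn, fires projectiles and is destroyed when its health runs out.
; PawnSensing starts AI movement toward the pawn to within attack range, or toward the "Exit"-tagged actor when the player enters FleeRange.
; Attacks turn to face the pawn and spawn from ProjectileSpawnPos on a timer-reset cooldown.
; BeginPlay sets damage by level; player distance tracking is incomplete and DamagePlayer is empty.
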(event `self.ReceiveTick`
  (params (DeltaSeconds :type "Float (single-precision)"))
  ;[1 1 1] Update - Move
  (if (not (`self.isSeeingPlayer`))
    (`MovementComponent.StopMovementImmediately` (`self.CharacterMovement`))
    (`self.Get Distance`)))

(event `self.PawnSensing.OnSeePawn`
  (params (Pawn :type "Pawn Object Reference"))
  ;[1 1 1] On See Pawn
  (set `self.Pawn` Pawn)
  (set `self.isSeeingPlayer` true)
  (`self.Follow Player`))

(event `self.ReceiveBeginPlay`
  (bind _stats (`self.Stats`))
  (bind ((`Level_13_B0432F0149067147026B04B503074291` _level)) (break `/Game/Carlos/Enemies/Enum/S_EnemyStats` _stats))
  ;[1 1 1] Set Level Damage
  (if (== _level 1)
    (bind _outactors (`GameplayStatics.GetAllActorsWithTag` "Exit" :!label _label))
    (set `self.Exit` (`|GetArrayItem` _outactors))
    (elif (== _level 2)
      (setmembers `/Game/Carlos/Enemies/Enum/S_EnemyStats` :`StructRef` _stats :`Damage` 8)
      (goto _label)
      (elif (== _level 3)
        (setmembers `/Game/Carlos/Enemies/Enum/S_EnemyStats` :`StructRef` _stats :`Damage` 10)
        (goto _label)))))

(event `Follow Player`
  ;[1 1 1] Follow Player
  (if (`self.isSeeingPlayer`)
    (if (`self.FleeRange`)
      (set `self.Move To` (`SceneComponent.K2_GetComponentLocation` (`Actor.RootComponent` (`self.Exit`))))
      (else
        (set `self.Move To` (`self.K2_GetActorLocation` (`self.Pawn`)))))
    (`|AIMoveTo` self (`self.Move To`) null (`.Range_15_AE6CF24E42D6FB128A62ADA5D6FE1211` (break `/Game/Carlos/Enemies/Enum/S_EnemyStats` (`self.Stats`)))
      (:`then`
        _)
      (:`OnSuccess`
        (set `self.InRange` true)))
    (`self.Attack`)
    (else
      (set `self.isSeeingPlayer` false))))

(event `Damage Enemy`
  (bind _stats (`self.Stats`))
  (bind ((`Health_12_D48A8CF14ACF631928A12998109E21C0` _health)) (break `/Game/Carlos/Enemies/Enum/S_EnemyStats` _stats))
  ;[1 1 1] Damage Enemy
  (setmembers `/Game/Carlos/Enemies/Enum/S_EnemyStats` :`StructRef` _stats :`Health` (- _health 1))
  (if (<= _health 0)
    (`self.K2_DestroyActor`)))

(event `Attack`
  ;[1 1 1] Attack
  (`self.Look At Player`)
  (if (`self.InRange`)
    (if (== (`self.AttackOnCD`) false)
      (set `self.AttackOnCD` true)
      (`|SpawnActorFromClass` "/Game/Carlos/Enemies/Blueprints/BP_LobberProjectile.BP_LobberProjectile_C" (`SceneComponent.K2_GetComponentToWorld` (`self.Projectile Spawn Pos`)) "AdjustIfPossibleButAlwaysSpawn" "OverrideRootScale" null null)
      (`KismetSystemLibrary.K2_SetTimer` null "ResetCD" (`self.AttackSpeed`)))))

(event `self.Flee Range.OnComponentBeginOverlap`
  (params (OverlappedComponent :type "PrimitiveComponent Object Reference") (OtherActor :type "Actor Object Reference") (OtherComp :type "PrimitiveComponent Object Reference") (OtherBodyIndex :type Integer) (bFromSweep :type Boolean) (SweepResult :type "HitResult Structure (by ref)"))
  (if (== (`KismetSystemLibrary.GetDisplayName` OtherActor) "DefaultPawn")
    (set `self.FleeRange` true)))

(event `ResetCD`
  ;[1 1 1] Attack
  (set `self.AttackOnCD` false))

(event `self.Flee Range.OnComponentEndOverlap`
  (params (OverlappedComponent :type "PrimitiveComponent Object Reference") (OtherActor :type "Actor Object Reference") (OtherComp :type "PrimitiveComponent Object Reference") (OtherBodyIndex :type Integer))
  (if (== (`KismetSystemLibrary.GetDisplayName` OtherActor) "DefaultPawn")
    (set `self.FleeRange` false)
    (`KismetSystemLibrary.Delay` 1.2)
    (`MovementComponent.StopMovementImmediately` (`self.CharacterMovement`))
    (`self.Follow Player`)))

(event `Damage Player`)

(event `Delete Sphere Collider`
  ;[1 1 1] Delete Sphere Comp
  (`KismetSystemLibrary.Delay` 0.5)
  (`ActorComponent.K2_DestroyComponent` (`self.Sphere`)))

(event `Look At Player`
  (bind _capsulecomponent (`self.CapsuleComponent`))
  (bind (_returnvalue_location _returnvalue_rotation _returnvalue_scale) (`KismetMathLibrary.BreakTransform` (`SceneComponent.K2_GetComponentToWorld` _capsulecomponent)))
  ;[1 1 1] Look at Player
  (bind _output_get (set `self.Look At Rotation` (`KismetMathLibrary.MakeTransform` _returnvalue_location (`KismetMathLibrary.FindLookAtRotation` (`SceneComponent.K2_GetComponentLocation` _capsulecomponent) (`SceneComponent.K2_GetComponentLocation` (`Actor.RootComponent` (`self.Pawn`)))) _returnvalue_scale)))
  (`self.K2_SetActorTransform` _output_get true))

(event `self.Sphere.OnComponentBeginOverlap`
  (params (OverlappedComponent :type "PrimitiveComponent Object Reference") (OtherActor :type "Actor Object Reference") (OtherComp :type "PrimitiveComponent Object Reference") (OtherBodyIndex :type Integer) (bFromSweep :type Boolean) (SweepResult :type "HitResult Structure (by ref)"))
  ;[1 1 1] Set Player Vars
  (if (`self.ActorHasTag` "Key")
    _
    (elif (`self.ActorHasTag` OtherActor "Elf")
      (set `self.Elf` OtherActor)
      (elif (`self.ActorHasTag` OtherActor "Valk")
        (set `self.Valk` OtherActor)
        (elif (`self.ActorHasTag` "Wizard")
          (set `self.Wizard` OtherActor)
          (elif (`self.ActorHasTag` "Warrior")
            (set `self.Warrior` OtherActor)))))))

(event `Get Distance`
  ;[1 1 1] SEt Distnances\
  (bind _aself_bp (cast `/Game/Players/Elf_Bp` (`self.Elf`)))
  (setmembers `/Game/Carlos/Enemies/Enum/S_Distance` :`StructRef` (`self.Distances`) :`DisValk` (`self.GetDistanceTo` self null) :`DisWarrior` (`self.GetDistanceTo` self null) :`DisWizard` (`self.GetDistanceTo` self null) :`DisElf` (`self.GetDistanceTo` self _aself_bp)))

(fn `UserConstructionScript`)