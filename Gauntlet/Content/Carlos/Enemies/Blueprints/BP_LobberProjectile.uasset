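; BP_LobberProjectile is the projectile fired by a lobber enemy that damages the player on contact.
; When its sphere overlaps a Bp_Player_Class actor, it subtracts ProjDamage directly from the player's Hp and destroys itself.
; A timer started on BeginPlay calls the same Damage event, which only destroys the actor, as a self-destruct after a set lifetime.
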(event `Damage`
  (`self.K2_DestroyActor`))

(event `self.ReceiveBeginPlay`
  (`KismetSystemLibrary.K2_SetTimer` null "Damage" (`self.SelfDestrucTimer`)))

(event `self.Sphere1.OnComponentBeginOverlap`
  (params (OverlappedComponent :type "PrimitiveComponent Object Reference") (OtherActor :type "Actor Object Reference") (OtherComp :type "PrimitiveComponent Object Reference") (OtherBodyIndex :type Integer) (bFromSweep :type Boolean) (SweepResult :type "HitResult Structure (by ref)"))
  (bind _asbp_player_class (cast `/Game/Players/Bp_Player_Class` OtherActor))
  (set `/Game/Players/Bp_Player_Class.Hp` (- (`/Game/Players/Bp_Player_Class.Hp` _asbp_player_class) (`self.projDamage`)) _asbp_player_class)
  (`self.Damage`))

(fn `UserConstructionScript`)