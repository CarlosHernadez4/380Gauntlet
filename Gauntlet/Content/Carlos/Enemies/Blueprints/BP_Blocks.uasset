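; BP_Blocks is a destructible enemy spawner that repeatedly produces one type of enemy.
; On BeginPlay it maps the enemy type in BlockStat to a Ghost, Grunt, Demon, Sorcerer or Lobber class.
; A looping timer spawns enemies at random X/Y points around the sphere range at the cube's height, with a cast chain for assigning the block's level.
; Projectiles overlapping the box are destroyed and reduce block health, destroying it at zero.
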(event `self.ReceiveBeginPlay`
  (`self.ChangeSpawnClass`)
  (`self.Spawn Enemy`))

(event `Spawn Enemy`
  (bind _spehre_spawn_range (`self.Spehre Spawn Range`))
  (bind ((`Level_13_B0432F0149067147026B04B503074291` _level)) (break `/Game/Carlos/Enemies/Enum/S_EnemyStats` (`self.BlockStat`)))
  (bind (_returnvalue_x _returnvalue_y _returnvalue_z) (`KismetMathLibrary.BreakVector` (`SceneComponent.K2_GetComponentLocation` (`self.Cube`))))
  (bind (_returnvalue_x_2 _returnvalue_y_2) (`KismetMathLibrary.BreakVector` (`KismetMathLibrary.RandomPointInBoundingBox` (`SceneComponent.K2_GetComponentLocation` _spehre_spawn_range) (`KismetMathLibrary.Conv_DoubleToVector` (`SphereComponent.GetScaledSphereRadius` _spehre_spawn_range)))))
  (bind _returnvalue (`|SpawnActorFromClass` (`self.Spawn Class`) (`KismetMathLibrary.MakeTransform` (`KismetMathLibrary.MakeVector` _returnvalue_x_2 _returnvalue_y_2 _returnvalue_z)) "AdjustIfPossibleButAlwaysSpawn" "OverrideRootScale" null null))
  (bind _asbp_ghost (cast `/Game/Carlos/Enemies/Blueprints/BP_Ghost` _returnvalue)
    (:`then`
      (bind _structout (setmembers `/Game/Carlos/Enemies/Enum/S_EnemyStats` :`StructRef` (`/Game/Carlos/Enemies/Blueprints/BP_Ghost.Stats` _asbp_ghost) :`Level` _level))
      (set `/Game/Carlos/Enemies/Blueprints/BP_Ghost.Stats` _structout _asbp_ghost))
    (:`CastFailed`
      (bind _asbp_grunts (cast `/Game/Carlos/Enemies/Blueprints/BP_Grunts` _returnvalue)
        (:`then`
          (bind _structout_2 (setmembers `/Game/Carlos/Enemies/Enum/S_EnemyStats` :`StructRef` (`/Game/Carlos/Enemies/Blueprints/BP_Grunts.Stats` _asbp_grunts) :`Level` _level))
          (set `/Game/Carlos/Enemies/Blueprints/BP_Grunts.Stats` _structout_2 _asbp_grunts))
        (:`CastFailed`
          (bind _asbp_demons (cast `/Game/Carlos/Enemies/Blueprints/BP_Demons` _returnvalue)
            (:`then`
              (setmembers `/Game/Carlos/Enemies/Enum/S_EnemyStats` :`StructRef` (`/Game/Carlos/Enemies/Blueprints/BP_Demons.Stats` _asbp_demons) :`Level` _level)
              (set `/Game/Carlos/Enemies/Blueprints/BP_Demons.Stats` (struct) _asbp_demons))
            (:`CastFailed`
              (bind _asbp_sorcerer (cast `/Game/Carlos/Enemies/Blueprints/BP_Sorcerer` _returnvalue)
                (:`then`
                  (bind _structout_3 (setmembers `/Game/Carlos/Enemies/Enum/S_EnemyStats` :`StructRef` (`/Game/Carlos/Enemies/Blueprints/BP_Sorcerer.Stats` _asbp_sorcerer) :`Level` _level))
                  (set `/Game/Carlos/Enemies/Blueprints/BP_Sorcerer.Stats` _structout_3 _asbp_sorcerer))
                (:`CastFailed`
                  (bind _asbp_lobbers (cast `/Game/Carlos/Enemies/Blueprints/BP_Lobbers` _returnvalue))
                  (bind _structout_4 (setmembers `/Game/Carlos/Enemies/Enum/S_EnemyStats` :`StructRef` (`/Game/Carlos/Enemies/Blueprints/BP_Lobbers.Stats` _asbp_lobbers) :`Level` _level))
                  (set `/Game/Carlos/Enemies/Blueprints/BP_Lobbers.Stats` _structout_4 _asbp_lobbers)))))))))
  (`KismetSystemLibrary.K2_SetTimer` null "Spawn Enemy" (`self.SpawnRate`) true))

(event `ChangeSpawnClass`
  (bind ((`EnemyType_2_ED4A4E914A448F8791ED5798B541B178` _enemytype)) (break `/Game/Carlos/Enemies/Enum/S_EnemyStats` (`self.BlockStat`)))
  (if (`|EnumEquality` _enemytype "NewEnumerator0")
    (set `self.Spawn Class` "/Game/Carlos/Enemies/Blueprints/BP_Ghost.BP_Ghost_C")
    (elif (`|EnumEquality` _enemytype "NewEnumerator1")
      (set `self.Spawn Class` "/Game/Carlos/Enemies/Blueprints/BP_Grunts.BP_Grunts_C")
      (elif (`|EnumEquality` _enemytype "NewEnumerator2")
        (set `self.Spawn Class` "/Game/Carlos/Enemies/Blueprints/BP_Demons.BP_Demons_C")
        (elif (`|EnumEquality` _enemytype "NewEnumerator3")
          (set `self.Spawn Class` "/Game/Carlos/Enemies/Blueprints/BP_Sorcerer.BP_Sorcerer_C")
          (elif (`|EnumEquality` _enemytype "NewEnumerator4")
            (set `self.Spawn Class` "/Game/Carlos/Enemies/Blueprints/BP_Lobbers.BP_Lobbers_C")))))))

(event `self.Box.OnComponentBeginOverlap`
  (params (OverlappedComponent :type "PrimitiveComponent Object Reference") (OtherActor :type "Actor Object Reference") (OtherComp :type "PrimitiveComponent Object Reference") (OtherBodyIndex :type Integer) (bFromSweep :type Boolean) (SweepResult :type "HitResult Structure (by ref)"))
  ;[1 1 1] Detect Projectile
  (bind _asbp_projectal (cast `/Game/Players/Bp_Projectal` OtherActor))
  (`self.Damage Bones`)
  (`self.K2_DestroyActor` _asbp_projectal))

(event `Damage Bones`
  (bind _blockstat (`self.BlockStat`))
  (bind ((`Health_12_D48A8CF14ACF631928A12998109E21C0` _health)) (break `/Game/Carlos/Enemies/Enum/S_EnemyStats` _blockstat))
  ;[1 1 1] Damage Bones
  (setmembers `/Game/Carlos/Enemies/Enum/S_EnemyStats` :`StructRef` _blockstat :`Health` (- _health 1))
  (if (<= _health 0)
    (`self.K2_DestroyActor`)))

(fn `UserConstructionScript`)