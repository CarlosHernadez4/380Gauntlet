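; Player character Blueprint that handles first-level controls: movement, camera look and shooting.
; Axis inputs add movement along the capsule's forward and right vectors, and feed yaw and pitch to the controller.
; BeginPlay creates the Ui widget and adds it to the viewport.
; Left mouse press spawns a Bp_Projectal at the SpawnProjectile component's location and rotation with an overridden scale, always spawning regardless of collision.
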(event `InputAxis|Up&Down`
  (params (AxisValue :type "Float (single-precision)"))
  ;[1 1 1] Movement
  (`self.AddMovementInput` (`SceneComponent.GetForwardVector` (`self.CapsuleComponent`)) AxisValue))

(event `InputAxis|Turn`
  (params (AxisValue :type "Float (single-precision)"))
  ;[1 1 1] Camra
  (`self.AddControllerYawInput` AxisValue))

(event `InputAxis|Left Rigth`
  (params (AxisValue :type "Float (single-precision)"))
  ;[1 1 1] Movement
  (`self.AddMovementInput` (`SceneComponent.GetRightVector` (`self.CapsuleComponent`)) AxisValue))

(event `InputAxis|Look Up`
  (params (AxisValue :type "Float (single-precision)"))
  ;[1 1 1] Camra
  (`self.AddControllerPitchInput` AxisValue))

(event `self.ReceiveBeginPlay`
  ;[1 1 1] Add Ui
  (bind _returnvalue (`|CreateWidget` "/Game/Players/Ui.Ui_C"))
  (`UserWidget.AddToViewport` _returnvalue 0))

(event `Key|LeftMouseButton`
  (params (Key :type "Key Structure"))
  (bind (_returnvalue_location _returnvalue_rotation) (`KismetMathLibrary.BreakTransform` (`SceneComponent.K2_GetComponentToWorld` (`self.Spawn Projectile`))))
  (:`Pressed`
    (`|SpawnActorFromClass` "/Game/Players/Bp_Projectal.Bp_Projectal_C" (`KismetMathLibrary.MakeTransform` _returnvalue_location _returnvalue_rotation (1.0 -0.25 -0.25)) "AlwaysSpawn" "OverrideRootScale" null null)))

(fn `UserConstructionScript`)